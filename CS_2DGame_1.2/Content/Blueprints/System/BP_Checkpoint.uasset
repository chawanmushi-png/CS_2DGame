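; BP_Checkpoint is a one-time checkpoint trigger that records where the player crosses it.
; When the player character first overlaps its Box, it sets a crossed flag and stores the character movement's last update location as the checkpoint location.
; It then turns on its point light and prints the saved location as debug text.
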(event `self.Box.OnComponentBeginOverlap`
  (params (OverlappedComponent :type "PrimitiveComponent Object Reference") (OtherActor :type "Actor Object Reference") (OtherComp :type "PrimitiveComponent Object Reference") (OtherBodyIndex :type Integer) (bFromSweep :type Boolean) (SweepResult :type "HitResult Structure (by ref)"))
  (bind _returnvalue (`GameplayStatics.GetPlayerCharacter` 0))
  (if (== OtherActor _returnvalue)
    (if (not (`self.CrossedCheckpoint`))
      (set `self.CrossedCheckpoint` true)
      (bind _output_get (set `self.CheckpointLocation` (`CharacterMovementComponent.GetLastUpdateLocation` (`Character.CharacterMovement` _returnvalue))))
      (`SceneComponent.SetVisibility` (`self.PointLight`) true false)
      (`KismetSystemLibrary.PrintString` (`KismetStringLibrary.Concat_StrStr` "Checkpoint saved at " (`KismetStringLibrary.Conv_VectorToString` _output_get)))
      (`KismetSystemLibrary.PrintString` (`KismetStringLibrary.Conv_VectorToString` (`self.CheckpointLocation`))))))

(fn `UserConstructionScript`)