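; Side-scroller skeleton enemy with a sprite, clamped health and a behavior-tree AI that hurts the player on contact.
; AnyDamage jumps the animation to damaged or dead; death sets the Blackboard's IsDead key and destroys the capsule.
; Hit deals damage and knocks the player back along the hit normal's X axis.
; Input movement flips the sprite, while the player-spotting reaction and test input-mapping setup are disconnected and never run.
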(event `self.ReceiveBeginPlay`
  (bind _asbp_warrior (cast `/Game/Blueprints/Warrior/BP_Warrior` (`GameplayStatics.GetPlayerCharacter` 0)))
  (set `self.castBP Warrior` _asbp_warrior)
  ;[1 1 1] Set Current Health to Max Health beginning of play
  (bind _output_get (set `self.fSkeletonCurrentHealth` (`self.fSkeletonMaxHealth`))))

(event `EnhancedInput|/Game/Blueprints/Input/Actions/IA_Movement`
  (params (ActionValue :type "Float (double-precision)") (ElapsedSeconds :type "Float (double-precision)") (TriggeredSeconds :type "Float (double-precision)") (InputAction :type "InputAction Object Reference" :default "/Game/Blueprints/Input/Actions/IA_Movement.IA_Movement"))
  (bind _sprite (`self.Sprite`))
  ;[1 1 1] Movement and character rotation
  (:`Triggered`
    (if (not (`self.bIsMovementLocked`))
      (`self.AddMovementInput` (`self.GetActorForwardVector`) ActionValue)
      (if (> ActionValue 0.0)
        (`SceneComponent.K2_SetWorldRotation` :`self` _sprite)
        (else
          (`SceneComponent.K2_SetWorldRotation` _sprite (struct :`Yaw` 180.0) false false))))))

(event `self.ReceiveAnyDamage`
  (params (Damage :type "Float (single-precision)") (DamageType :type "DamageType Object Reference") (InstigatedBy :type "Controller Object Reference") (DamageCauser :type "Actor Object Reference"))
  ;[1 1 1] Damage
  (if (not (`self.bIsDead`))
    (set `self.bIsMovementLocked` true)
    (bind _output_get (set `self.fSkeletonCurrentHealth` (`KismetMathLibrary.FClamp` (- (`self.fSkeletonCurrentHealth`) Damage) 0.0 (`self.fSkeletonMaxHealth`))))
    (if (<= (`self.fSkeletonCurrentHealth`) 0.0)
      (`PaperZDAnimInstance.JumpToNode` (`PaperZDAnimationComponent.AnimInstance` (`self.AnimationComponent`)) "EnemySkeleton_Dead" "None")
      (`KismetSystemLibrary.PrintString` "Skeleton Dies" true true (struct :`R` 1.0 :`B` 0.007843 :`A` 1.0) 4.0)
      (set `self.bIsDead` true)
      (`BlackboardComponent.SetValueAsBool` (`AIBlueprintHelperLibrary.GetBlackboard` (`AIBlueprintHelperLibrary.GetAIController` self)) "IsDead" true) ; Sets IsDead key to true on BT_EnemySkeleton, disabling behavior trees
      (`ActorComponent.K2_DestroyComponent` (`self.CapsuleComponent`))
      (else
        (`PaperZDAnimInstance.JumpToNode` (`PaperZDAnimationComponent.AnimInstance` (`self.AnimationComponent`)) "EnemySkeleton_Damaged" "None")
        (set `self.bIsMovementLocked` false)
        (`KismetSystemLibrary.PrintString` (`KismetStringLibrary.Concat_StrStr` "Hit! Skeleton's health is now " (`KismetStringLibrary.Conv_DoubleToString` _output_get)) true true (struct :`R` 1.0 :`B` 0.007843 :`A` 1.0) 4.0)))))

(event `self.ReceiveHit`
  (params (MyComp :type "PrimitiveComponent Object Reference") (Other :type "Actor Object Reference") (OtherComp :type "PrimitiveComponent Object Reference") (bSelfMoved :type Boolean) (HitLocation :type "Vector Structure") (HitNormal :type "Vector Structure") (NormalImpulse :type "Vector Structure") (Hit :type "HitResult Structure (by ref)"))
  (bind _returnvalue (`GameplayStatics.GetPlayerCharacter` 0))
  ;[1 1 1] Player Event Hit damage and knockback
  (if (== Other _returnvalue)
    (`GameplayStatics.ApplyDamage` _returnvalue 10.0)
    (`CharacterMovementComponent.AddImpulse` (`Character.CharacterMovement` _returnvalue) (* HitNormal (-2000.0 0.0 0.0)) true)))

(fn `UserConstructionScript`)