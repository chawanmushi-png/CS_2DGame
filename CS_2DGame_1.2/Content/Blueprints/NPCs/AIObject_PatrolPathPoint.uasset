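; A patrol path point that orients a patrolling character along its arrow when the character arrives.
; An entered event stores the character, opens a gate and fires an OnPointMet dispatcher for other logic to react to.
; While the gate is open, Tick eases the character's rotation toward the arrow's world rotation, until the exit event closes it.
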(event `self.ReceiveTick`
  (params (DeltaSeconds :type "Float (single-precision)"))
  (`/Engine/EditorBlueprintResources/StandardMacros.Gate` true :!label _label
    (:`Exit`
      (`self.K2_SetActorRotation` (`self.C Character`) (`KismetMathLibrary.RInterpTo` (`self.K2_GetActorRotation` (`self.C Character`)) (`SceneComponent.K2_GetComponentRotation` (`self.Arrow`)) DeltaSeconds 2.0) false))))

(event `On Patroller Exit`
  (goto _label :!via `Close`))

(event `OnPatrollerEntered`
  (params (cCharacter :type "Character Object Reference"))
  (set `self.C Character` cCharacter)
  (`|ExecutionSequence`
    (:`then_0`
      (goto _label :!via `Open`))
    (:`then_1`
      (`self.OnPointMet`) ; Can be called by other events to trigger something when pawn reaches point
    )))

(fn `UserConstructionScript`)