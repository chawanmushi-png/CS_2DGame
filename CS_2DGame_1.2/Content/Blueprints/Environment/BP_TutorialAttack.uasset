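; A placeable trigger that shows an attack tutorial widget while the player character stands inside its box.
; On BeginPlay it creates WBP_TutorialAttack, adds it to the viewport and hides it.
; Entering the box makes the widget visible and plays its fade-in animation.
; Leaving plays the fade-out after a short delay, then hides the widget after a further delay.
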(event `self.ReceiveBeginPlay`
  (bind _returnvalue (`|CreateWidget` "/Game/Blueprints/Environment/Widgets/WBP_TutorialAttack.WBP_TutorialAttack_C"))
  (bind _output_get (set `self.TutorialAttack` _returnvalue))
  (`UserWidget.AddToViewport` _output_get 0)
  (`Widget.SetVisibility` _output_get "Hidden"))

(event `self.Box.OnComponentBeginOverlap`
  (params (OverlappedComponent :type "PrimitiveComponent Object Reference") (OtherActor :type "Actor Object Reference") (OtherComp :type "PrimitiveComponent Object Reference") (OtherBodyIndex :type Integer) (bFromSweep :type Boolean) (SweepResult :type "HitResult Structure (by ref)"))
  (bind _tutorialattack (`self.TutorialAttack`))
  (if (== OtherActor (`GameplayStatics.GetPlayerCharacter` 0))
    (`Widget.SetVisibility` _tutorialattack "Visible")
    (`UserWidget.PlayAnimation` _tutorialattack (`/Game/Blueprints/Environment/Widgets/WBP_TutorialAttack.FadeIn` _tutorialattack) 0.0 1 "Forward" 1.0 false)))

(event `self.Box.OnComponentEndOverlap`
  (params (OverlappedComponent :type "PrimitiveComponent Object Reference") (OtherActor :type "Actor Object Reference") (OtherComp :type "PrimitiveComponent Object Reference") (OtherBodyIndex :type Integer))
  (bind _tutorialattack (`self.TutorialAttack`))
  (if (== OtherActor (`GameplayStatics.GetPlayerCharacter` 0))
    (`KismetSystemLibrary.Delay` 0.2)
    (`UserWidget.PlayAnimation` _tutorialattack (`/Game/Blueprints/Environment/Widgets/WBP_TutorialAttack.FadeOut` _tutorialattack) 0.0 1 "Forward" 1.0 false)
    (`KismetSystemLibrary.Delay` 1.0)
    (`Widget.SetVisibility` (`self.TutorialAttack`) "Hidden")))

(fn `UserConstructionScript`)