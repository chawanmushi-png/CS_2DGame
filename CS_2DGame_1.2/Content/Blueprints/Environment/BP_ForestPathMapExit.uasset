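; Forest path exit trigger that shows exit and interact prompts when the player enters its box, apparently intended as a map transition.
; Overlap events fade the exit prompt, toggle the interact widget and open or close a gate; both enable input.
; IA_Interact drives a progress animation and a gated, do-once hold.
; The hold ends at a delay, leaving the Map_GloomForest level load disconnected.
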(event `self.ReceiveBeginPlay`
  (bind _returnvalue (`|CreateWidget` "/Game/Blueprints/Environment/Widgets/WBP_ForestPathExitPrompt.WBP_ForestPathExitPrompt_C"))
  (bind _output_get (set `self.ForestPathExitPrompt` _returnvalue))
  (`UserWidget.AddToViewport` _output_get 0)
  (`Widget.SetVisibility` _output_get "Hidden")
  (bind _returnvalue_2 (`|CreateWidget` "/Game/Blueprints/System/Widgets/WBP_InteractDisplay.WBP_InteractDisplay_C"))
  (bind _output_get_2 (set `self.WidgetInteract` _returnvalue_2))
  (`UserWidget.AddToViewport` _output_get_2 0))

(event `EnhancedInput|/Game/Blueprints/Input/Actions/IA_Interact`
  (params (ActionValue :type Boolean) (ElapsedSeconds :type "Float (double-precision)") (TriggeredSeconds :type "Float (double-precision)") (InputAction :type "InputAction Object Reference" :default "/Game/Blueprints/Input/Actions/IA_Interact.IA_Interact"))
  (bind _widgetinteract (`self.WidgetInteract`))
  (bind _interactprogressanimation (`/Game/Blueprints/System/Widgets/WBP_InteractDisplay.InteractProgressAnimation` _widgetinteract))
  (:`Triggered`
    (`/Engine/EditorBlueprintResources/StandardMacros.DoOnce` false :!label _label
      (:`Completed`
        (set `self.InteractHeld` ActionValue)
        (`/Engine/EditorBlueprintResources/StandardMacros.Gate` true :!label _label_2
          (:`Exit`
            (`/Engine/EditorBlueprintResources/StandardMacros.DoOnce` false
              (:`Completed`
                (`KismetSystemLibrary.Delay` 0.2))))))))
  (:`Started`
    (`UserWidget.PlayAnimation` _widgetinteract _interactprogressanimation 0.0 1 "Forward" 1.0 false))
  (:`Canceled`
    (`UserWidget.StopAnimation` _widgetinteract _interactprogressanimation)
    (goto _label :!via `Reset`))
  (:`Completed`
    (set `self.InteractHeld` false)
    (`KismetSystemLibrary.Delay` 0.2)
    (`Widget.SetVisibility` _widgetinteract "Hidden")
    (goto _label :!via `Reset`)))

(event `self.Box.OnComponentBeginOverlap`
  (params (OverlappedComponent :type "PrimitiveComponent Object Reference") (OtherActor :type "Actor Object Reference") (OtherComp :type "PrimitiveComponent Object Reference") (OtherBodyIndex :type Integer) (bFromSweep :type Boolean) (SweepResult :type "HitResult Structure (by ref)"))
  (bind _forestpathexitprompt (`self.ForestPathExitPrompt`))
  (if (== OtherActor (`GameplayStatics.GetPlayerCharacter` 0))
    (`Widget.SetVisibility` (`self.WidgetInteract`) "Visible")
    (`Widget.SetVisibility` _forestpathexitprompt "Visible")
    (`UserWidget.PlayAnimation` _forestpathexitprompt (`/Game/Blueprints/Environment/Widgets/WBP_ForestPathExitPrompt.FadeIn` _forestpathexitprompt) 0.0 1 "Forward" 1.0 false)
    (`self.EnableInput` (`GameplayStatics.GetPlayerController` 0))
    (goto _label_2 :!via `Open`)))

(event `self.Box.OnComponentEndOverlap`
  (params (OverlappedComponent :type "PrimitiveComponent Object Reference") (OtherActor :type "Actor Object Reference") (OtherComp :type "PrimitiveComponent Object Reference") (OtherBodyIndex :type Integer))
  (bind _forestpathexitprompt (`self.ForestPathExitPrompt`))
  (if (== (`GameplayStatics.GetPlayerCharacter` 0) OtherActor)
    (`Widget.SetVisibility` (`self.WidgetInteract`) "Hidden")
    (`KismetSystemLibrary.Delay` 0.2)
    (`UserWidget.PlayAnimation` _forestpathexitprompt (`/Game/Blueprints/Environment/Widgets/WBP_ForestPathExitPrompt.FadeOut` _forestpathexitprompt) 0.0 1 "Forward" 1.0 false)
    (`KismetSystemLibrary.Delay` 1.0)
    (`Widget.SetVisibility` _forestpathexitprompt "Hidden")
    (`self.EnableInput` (`GameplayStatics.GetPlayerController` 0))
    (goto _label_2 :!via `Close`)))

(fn `UserConstructionScript`)