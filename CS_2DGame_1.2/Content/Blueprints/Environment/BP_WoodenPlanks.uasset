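; BP_WoodenPlanks is a destructible environment actor that takes damage and is removed when its health runs out.
; Health starts at MaxHealth, and AnyDamage subtracts from it with a clamp between zero and that maximum.
; Each hit briefly plays the BeamFlashFlipBook flash, and the zero-health check runs only after that delay.
; At zero, it sets IsDestroyed to ignore further damage and calls BeamsBroken, which destroys the actor.
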(event `self.ReceiveBeginPlay`
  (set `self.CurrentHealth` (`self.MaxHealth`)))

(event `self.ReceiveAnyDamage`
  (params (Damage :type "Float (single-precision)") (DamageType :type "DamageType Object Reference") (InstigatedBy :type "Controller Object Reference") (DamageCauser :type "Actor Object Reference"))
  (bind _beamflashflipbook (`self.BeamFlashFlipBook`))
  (if (not (`self.IsDestroyed`))
    (set `self.CurrentHealth` (`KismetMathLibrary.FClamp` (- (`self.CurrentHealth`) Damage) 0.0 (`self.MaxHealth`)))
    (`SceneComponent.SetVisibility` _beamflashflipbook true false)
    (`PaperFlipbookComponent.PlayFromStart` _beamflashflipbook)
    (`KismetSystemLibrary.Delay` 0.25)
    (`SceneComponent.SetVisibility` _beamflashflipbook false false)
    (if (<= (`self.CurrentHealth`) 0.0)
      (set `self.IsDestroyed` true)
      (`self.Beams Broken`))))

(event `Beams Broken`
  (`self.K2_DestroyActor`))

(fn `UserConstructionScript`)