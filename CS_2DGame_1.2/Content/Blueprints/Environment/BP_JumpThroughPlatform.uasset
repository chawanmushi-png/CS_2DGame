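; One-way platform that the BP_Warrior player can jump up through or drop down through.
; Overlapping the bottom collider disables MainPlatform collision, and leaving it restores collision.
; The top collider opens and closes a gate that lets the IA_FallThroughPlatforms input disable collision, which only the bottom collider's end overlap restores.
; The construction script applies sprite, scale and rotation to the platform.
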(event `self.ReceiveBeginPlay`
  (bind _asbp_warrior (cast `/Game/Blueprints/Warrior/BP_Warrior` (`GameplayStatics.GetPlayerCharacter` 0)))
  (set `self.cBPWarriorCapsuleComponent` (`Character.CapsuleComponent` _asbp_warrior)))

(event `EnhancedInput|/Game/Blueprints/Input/Actions/IA_FallThroughPlatforms`
  (params (ActionValue :type Boolean) (ElapsedSeconds :type "Float (double-precision)") (TriggeredSeconds :type "Float (double-precision)") (InputAction :type "InputAction Object Reference" :default "/Game/Blueprints/Input/Actions/IA_FallThroughPlatforms.IA_FallThroughPlatforms"))
  ;[1 1 1] Fall through platform on S keypress
  (:`Triggered`
    (`/Engine/EditorBlueprintResources/StandardMacros.Gate` true :!label _label
      (:`Exit`
        (`PrimitiveComponent.SetCollisionEnabled` (`self.MainPlatform`) "NoCollision")))))

(event `self.PlatformColliderTop.OnComponentBeginOverlap`
  (params (OverlappedComponent :type "PrimitiveComponent Object Reference") (OtherActor :type "Actor Object Reference") (OtherComp :type "PrimitiveComponent Object Reference") (OtherBodyIndex :type Integer) (bFromSweep :type Boolean) (SweepResult :type "HitResult Structure (by ref)"))
  ;[1 1 1] Fall through platform on S keypress
  (if (== OtherComp (`self.cBPWarriorCapsuleComponent`))
    (`self.EnableInput` (`GameplayStatics.GetPlayerController` 0))
    (goto _label :!via `Open`)))

(event `self.PlatformColliderTop.OnComponentEndOverlap`
  (params (OverlappedComponent :type "PrimitiveComponent Object Reference") (OtherActor :type "Actor Object Reference") (OtherComp :type "PrimitiveComponent Object Reference") (OtherBodyIndex :type Integer))
  ;[1 1 1] Fall through platform on S keypress
  (if (== (`self.cBPWarriorCapsuleComponent`) OtherComp)
    (`self.EnableInput` (`GameplayStatics.GetPlayerController` 0))
    (goto _label :!via `Close`)))

(event `self.PlatformColliderBot.OnComponentBeginOverlap`
  (params (OverlappedComponent :type "PrimitiveComponent Object Reference") (OtherActor :type "Actor Object Reference") (OtherComp :type "PrimitiveComponent Object Reference") (OtherBodyIndex :type Integer) (bFromSweep :type Boolean) (SweepResult :type "HitResult Structure (by ref)"))
  ;[1 1 1] Jump up through platform
  (if (== OtherComp (`self.cBPWarriorCapsuleComponent`))
    (`PrimitiveComponent.SetCollisionEnabled` (`self.MainPlatform`) "NoCollision")))

(event `self.PlatformColliderBot.OnComponentEndOverlap`
  (params (OverlappedComponent :type "PrimitiveComponent Object Reference") (OtherActor :type "Actor Object Reference") (OtherComp :type "PrimitiveComponent Object Reference") (OtherBodyIndex :type Integer))
  ;[1 1 1] Jump up through platform
  (if (== (`self.cBPWarriorCapsuleComponent`) OtherComp)
    (`PrimitiveComponent.SetCollisionEnabled` (`self.MainPlatform`) "QueryAndPhysics")))

(fn `UserConstructionScript`
  (bind _mainplatform (`self.MainPlatform`))
  (`PaperSpriteComponent.SetSprite` _mainplatform (`self.cPlatformSprite`))
  (`SceneComponent.SetRelativeScale3D` _mainplatform (`self.Scale`))
  (`SceneComponent.K2_SetRelativeRotation` _mainplatform (`self.Rotation`) false false))