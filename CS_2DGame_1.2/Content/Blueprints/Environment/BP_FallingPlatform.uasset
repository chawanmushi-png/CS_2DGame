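; A 2D sprite platform that drops while the player's BP_Warrior is on its trigger and recovers when the player leaves.
; Overlaps with the warrior's capsule play or reverse a timeline that lerps the platform between its start and end locations.
; Separate drop and recover durations set the timeline's play rate.
; The construction script applies sprite, scale and rotation to the platform and an end-position reference placed at the target location.
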(event `self.ReceiveBeginPlay`
  ;[1 1 1] Sets our v_StartLocation variable to our main platforms location at th start of game
  (set `self.v_Start Location` (`SceneComponent.RelativeLocation` (`self.MainPlatform`)))
  (bind _asbp_warrior (cast `/Game/Blueprints/Warrior/BP_Warrior` (`GameplayStatics.GetPlayerCharacter` 0)))
  (set `self.cBPWarriorCapsuleComponent` (`Character.CapsuleComponent` _asbp_warrior)))

(event `self.PlatformCollider.OnComponentBeginOverlap`
  (params (OverlappedComponent :type "PrimitiveComponent Object Reference") (OtherActor :type "Actor Object Reference") (OtherComp :type "PrimitiveComponent Object Reference") (OtherBodyIndex :type Integer) (bFromSweep :type Boolean) (SweepResult :type "HitResult Structure (by ref)"))
  ;[1 1 1] Sets a begin and end overlap event which sets the "play rate" of our moving platform's timeline (which goes from 0 - 1).
  (if (== OtherComp (`self.cBPWarriorCapsuleComponent`))
    (`TimelineComponent.SetPlayRate` (`self.Move Platform`) (/ 1.0 (`self.f_DropDuration(Seconds)`)))
    ;[1 1 1] We set a Timeline between 0 and 1 called Move Platform. 0 is equal to value A (v_StartLocation) in our Lerp (Vector) and 1 is equal to value B (v_EndLocation). The return value of our Lerp will define our SM_MainPlatform's new location.
    (bind (_direction _move_track) (`Timeline|Move Platform` :!label _label)
      (:`Update`
        (`SceneComponent.K2_SetRelativeLocation` (`self.MainPlatform`) (`KismetMathLibrary.VLerp` (`self.v_Start Location`) (`self.v_EndLocation`) _move_track) false false)))))

(event `self.PlatformCollider.OnComponentEndOverlap`
  (params (OverlappedComponent :type "PrimitiveComponent Object Reference") (OtherActor :type "Actor Object Reference") (OtherComp :type "PrimitiveComponent Object Reference") (OtherBodyIndex :type Integer))
  ;[1 1 1] Sets a begin and end overlap event which sets the "play rate" of our moving platform's timeline (which goes from 0 - 1).
  (if (== (`self.cBPWarriorCapsuleComponent`) OtherComp)
    (`TimelineComponent.SetPlayRate` (`self.Move Platform`) (/ 1.0 (`self.f_RecoverDuration(Seconds)`)))
    (goto _label :!via `Reverse`)))

(fn `UserConstructionScript`
  (bind _endplatformreference (`self.EndPlatformReference`))
  (bind _platform_sprite (`self.Platform Sprite`))
  (`PaperSpriteComponent.SetSprite` (`self.MainPlatform`) _platform_sprite)
  (`PaperSpriteComponent.SetSprite` _endplatformreference _platform_sprite)
  (`SceneComponent.SetRelativeScale3D` _endplatformreference (`self.Scale`))
  (`SceneComponent.SetRelativeScale3D` (`self.MainPlatform`) (`self.Scale`))
  (`SceneComponent.K2_SetRelativeRotation` _endplatformreference (`self.Rotation`) false false)
  (`SceneComponent.K2_SetRelativeRotation` (`self.MainPlatform`) (`self.Rotation`) false false)
  (`SceneComponent.K2_SetRelativeLocation` _endplatformreference (`self.v_EndLocation`) false false))