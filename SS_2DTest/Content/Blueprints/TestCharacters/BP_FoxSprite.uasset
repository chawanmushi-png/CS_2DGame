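; BP_FoxSprite is a player-controlled 2D flipbook character with side-scrolling movement along world X and jumping.
; MoveRight and Jump input drive the character's movement.
; Each tick picks the fall, run or idle flipbook from falling state and velocity.
; It also sets controller yaw to 0 or 180 from X velocity to face the travel direction, keeping the last facing when X velocity is zero.
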(event `InputAxis|MoveRight`
  (params (AxisValue :type "Float (single-precision)"))
  (`self.AddMovementInput` (1.0 0.0 0.0) AxisValue))

(event `InputAction|Jump`
  (params (Key :type "Key Structure"))
  ;[1 1 1] Player Jump
  (:`Pressed`
    (`self.Jump`))
  (:`Released`
    (`self.StopJumping`)))

(event `self.ReceiveTick`
  (params (DeltaSeconds :type "Float (single-precision)"))
  (`self.UpdateAnimation`)
  (`self.UpdateControlRotation`))

(event `UpdateAnimation`
  ;[1 1 1] Check if Player is Moving, False sets Idle, True sets Run Flip Book
  (`PaperFlipbookComponent.SetFlipbook` (`self.Sprite`) (select `bool` (`NavMovementComponent.IsFalling` (`self.CharacterMovement`)) :`false` (select `bool` (> (`KismetMathLibrary.VSize` (`MovementComponent.Velocity` (`self.CharacterMovement`))) 0.0) :`false` "/Game/Assets/FB_Player_Idle.FB_Player_Idle" :`true` "/Game/Assets/FB_Player_Run.FB_Player_Run" :!type "PaperFlipbook Object Reference") :`true` "/Game/Assets/FB_Player_Fall.FB_Player_Fall")))

(event `UpdateControlRotation`
  ;[1 1 1] Update Character Facing Direction
  (`/Engine/EditorBlueprintResources/StandardMacros.IsValid` (`self.GetController`)
    (:`Is Valid`
      (`/Engine/EditorBlueprintResources/StandardMacros.CompareFloat` (.x (`MovementComponent.Velocity` (`self.CharacterMovement`)))
        (:`>`
          (`Controller.SetControlRotation` (`self.GetController`) (`KismetMathLibrary.MakeRotator` 0.0)))
        (:`<`
          (`Controller.SetControlRotation` (`self.GetController`) (`KismetMathLibrary.MakeRotator` 0.0 0.0 180.0)))))))

(fn `UserConstructionScript`)