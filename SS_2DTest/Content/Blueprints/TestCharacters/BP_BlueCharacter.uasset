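; Blue test Paper2D side-scroller character with run and jump, driven by Enhanced Input added on BeginPlay.
; Movement input runs along the actor's forward vector, swaps run/idle flipbooks and flips the sprite by input sign.
; Jumping locks movement input and plays a non-looping flipbook, then polls vertical velocity through a short Delay loop until zero to restore idle.
; An UpdateAnimation event selects fall, run or idle, but nothing in this graph calls it.
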(event `self.ReceiveBeginPlay`
  ;[1 1 1] Spawn PlayerController on Play
  (bind _asbp_player_controller (cast `/Game/Blueprints/BP_PlayerController` (`self.GetController`)))
  (`EnhancedInputSubsystemInterface.AddMappingContext` (pcsubsystem `EnhancedInputLocalPlayerSubsystem` _asbp_player_controller) "/Game/Blueprints/Input/IMC_Sidescroller.IMC_Sidescroller" 0 (struct)))

(event `EnhancedInput|/Game/Blueprints/Input/Actions/IA_Movement`
  (params (ActionValue :type "Float (double-precision)") (ElapsedSeconds :type "Float (double-precision)") (TriggeredSeconds :type "Float (double-precision)") (InputAction :type "InputAction Object Reference" :default "/Game/Blueprints/Input/Actions/IA_Movement.IA_Movement"))
  ;[1 1 1] Character Input Action - Movement
  (:`Triggered`
    (if (not (`self.bIsJumping`))
      ;;[1 1 1] Forward movement input and sets Run FB
      (`self.AddMovementInput` (`self.GetActorForwardVector`) ActionValue)
      (`PaperFlipbookComponent.SetFlipbook` (`self.Sprite`) "/Game/Assets/FB_CharBlue_Run.FB_CharBlue_Run")
      ;;[1 1 1] Looks at input action value, if value is greater than 0, then rotates sprite 180 degrees, turning them
      (if (> ActionValue 0.0)
        (`SceneComponent.K2_SetWorldRotation` :`self` (`self.Sprite`))
        (else
          (`SceneComponent.K2_SetWorldRotation` (`self.Sprite`) (struct :`Yaw` -180.0) false false)))))
  (:`Completed`
    (if (not (`self.bIsJumping`))
      ;;[1 1 1] Otherwise play Idle FB
      (`PaperFlipbookComponent.SetFlipbook` (`self.Sprite`) "/Game/Assets/FB_CharBlue_Idle.FB_CharBlue_Idle"))))

(event `EnhancedInput|/Game/Blueprints/Input/Actions/IA_Jump`
  (params (ActionValue :type Boolean) (ElapsedSeconds :type "Float (double-precision)") (TriggeredSeconds :type "Float (double-precision)") (InputAction :type "InputAction Object Reference" :default "/Game/Blueprints/Input/Actions/IA_Jump.IA_Jump"))
  (bind (_returnvalue_x _returnvalue_y _returnvalue_z) (`KismetMathLibrary.BreakVector` (`self.GetVelocity`)))
  (bind _sprite (`self.Sprite`))
  (:`Triggered`
    (if (not (`self.bIsJumping`))
      (set `self.bIsJumping` true)
      (`self.Jump`)
      ;[1 1 1] So jump animation doesn't loop
      (`PaperFlipbookComponent.SetLooping` _sprite false)
      (`PaperFlipbookComponent.SetFlipbook` _sprite "/Game/Assets/FB_CharBlue_Jump.FB_CharBlue_Jump")
      (`KismetSystemLibrary.Delay` 0.01)
      (if (== _returnvalue_z 0.0) :!label _label
        (`PaperFlipbookComponent.SetLooping` _sprite true)
        (`PaperFlipbookComponent.Play` _sprite)
        (`PaperFlipbookComponent.SetFlipbook` _sprite "/Game/Assets/FB_CharBlue_Idle.FB_CharBlue_Idle")
        (set `self.bIsJumping` false)
        (else
          (`KismetSystemLibrary.Delay` 0.01)
          (goto _label))))))

(event `UpdateAnimation`
  ;[1 1 1] Check if Player is Moving, False sets Idle, True sets Run Flip Book
  (`PaperFlipbookComponent.SetFlipbook` (`self.Sprite`) (select `bool` (`NavMovementComponent.IsFalling` (`self.CharacterMovement`)) :`false` (select `bool` (> (`KismetMathLibrary.VSize` (`MovementComponent.Velocity` (`self.CharacterMovement`))) 0.0) :`false` "/Game/Assets/FB_CharBlue_Idle.FB_CharBlue_Idle" :`true` "/Game/Assets/FB_CharBlue_Run.FB_CharBlue_Run" :!type "PaperFlipbook Object Reference") :`true` "/Game/Assets/FB_CharBlue_Fall.FB_CharBlue_Fall")))

(fn `UserConstructionScript`)