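; PaperZD anim notify for the Warrior's first light attack, applying sword hit damage when the notify fires.
; It runs a box overlap for Pawns at the SwordAttack1 socket on the render component, ignoring the owner, and applies fixed damage to each actor found, with debug prints.
; Without a valid owning instance, it draws a debug box of the same hit volume instead.
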(event `self.OnReceiveNotify`
  (params (OwningInstance :type "PaperZDAnimInstance Object Reference"))
  (bind _v_hitboxextent (`self.v_HitBoxExtent`))
  (bind _returnvalue (`SceneComponent.GetSocketLocation` (`self.SequenceRenderComponent`) "SwordAttack1"))
  (`/Engine/EditorBlueprintResources/StandardMacros.IsValid` OwningInstance
    (:`Is Valid`
      (bind _outactors (`KismetSystemLibrary.BoxOverlapActors` _returnvalue _v_hitboxextent (`|MakeArray` "ObjectTypeQuery3" :!type "EObjectTypeQuery Enum") null (`|MakeArray` (`PaperZDAnimInstance.GetOwningActor` OwningInstance))))
      (for _array_element _outactors
        (`KismetSystemLibrary.PrintString` (`KismetSystemLibrary.GetDisplayName` _array_element))
        (bind _returnvalue_2 (`GameplayStatics.ApplyDamage` _array_element 10.0))
        (`KismetSystemLibrary.PrintString` (`KismetStringLibrary.Concat_StrStr` "damage cast " (`KismetStringLibrary.Conv_DoubleToString` _returnvalue_2)) true true (struct :`R` 1.0 :`B` 0.007843 :`A` 1.0) 4.0))
      (`KismetSystemLibrary.PrintString` "No more actors found"))
    (:`Is Not Valid`
      (`KismetSystemLibrary.DrawDebugBox` _returnvalue _v_hitboxextent (struct :`R` 1.0 :`A` 1.0)))))