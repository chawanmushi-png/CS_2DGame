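; Shopkeeper NPC that shows dialogue when the player walks into its trigger box.
; BeginPlay creates a shopkeeper dialogue widget and adds it to the viewport hidden.
; On player overlap the widget fades in and, after a short delay, a speech bubble appears and plays from the start.
; When the player leaves, the widget fades out, then both widget and bubble hide after timed delays.
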(event `self.ReceiveBeginPlay`
  (bind _shopkeeper_dialogue_widget (`self.Shopkeeper Dialogue Widget`))
  (bind _returnvalue (`|CreateWidget` "/Game/Blueprints/NPCs/Widgets/WBP_ShopkeeperDialogueBox.WBP_ShopkeeperDialogueBox_C"))
  (set `self.Shopkeeper Dialogue Widget` _returnvalue)
  (`UserWidget.AddToViewport` _shopkeeper_dialogue_widget 0)
  (`Widget.SetVisibility` _shopkeeper_dialogue_widget "Hidden"))

(event `self.Box.OnComponentBeginOverlap`
  (params (OverlappedComponent :type "PrimitiveComponent Object Reference") (OtherActor :type "Actor Object Reference") (OtherComp :type "PrimitiveComponent Object Reference") (OtherBodyIndex :type Integer) (bFromSweep :type Boolean) (SweepResult :type "HitResult Structure (by ref)"))
  (bind _shopkeeper_dialogue_widget (`self.Shopkeeper Dialogue Widget`))
  (bind _fb_speechbubble (`self.FB_SpeechBubble`))
  (if (== OtherActor (`GameplayStatics.GetPlayerCharacter` 0))
    (`Widget.SetVisibility` _shopkeeper_dialogue_widget "Visible")
    (`UserWidget.PlayAnimation` _shopkeeper_dialogue_widget (`/Game/Blueprints/NPCs/Widgets/WBP_ShopkeeperDialogueBox.FadeIn` _shopkeeper_dialogue_widget) 0.0 1 "Forward" 1.0 false)
    (`KismetSystemLibrary.Delay` 0.2)
    (`SceneComponent.SetVisibility` _fb_speechbubble true false)
    (`PaperFlipbookComponent.PlayFromStart` _fb_speechbubble)))

(event `self.Box.OnComponentEndOverlap`
  (params (OverlappedComponent :type "PrimitiveComponent Object Reference") (OtherActor :type "Actor Object Reference") (OtherComp :type "PrimitiveComponent Object Reference") (OtherBodyIndex :type Integer))
  (bind _shopkeeper_dialogue_widget (`self.Shopkeeper Dialogue Widget`))
  (if (== OtherActor (`GameplayStatics.GetPlayerCharacter` 0))
    (`KismetSystemLibrary.Delay` 0.2)
    (`UserWidget.PlayAnimation` _shopkeeper_dialogue_widget (`/Game/Blueprints/NPCs/Widgets/WBP_ShopkeeperDialogueBox.FadeOut` _shopkeeper_dialogue_widget) 0.0 1 "Forward" 1.0 false)
    (`KismetSystemLibrary.Delay` 1.0)
    (`Widget.SetVisibility` (`self.Shopkeeper Dialogue Widget`) "Hidden")
    (`SceneComponent.SetVisibility` (`self.FB_SpeechBubble`) false false)))

(fn `UserConstructionScript`)