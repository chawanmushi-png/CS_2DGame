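; AI controller for the skeleton enemy that runs its behavior tree on BeginPlay and feeds it perception data through the Blackboard.
; Each perception update passes through separate sight and hearing handlers, filtered by sense class.
; Sight sets FoundPlayer to the player while seen, clears it when sight is lost, and stores PlayerLastKnownLocation.
; Hearing stores any noise position as HeardNoiseLocation, and both handlers print debug messages.
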(event `self.ReceiveBeginPlay`
  (`self.RunBehaviorTree` "/Game/Blueprints/NPCs/BT_EnemySkeleton.BT_EnemySkeleton"))

(event `self.AIPerception.OnTargetPerceptionUpdated`
  (params (Actor :type "Actor Object Reference") (Stimulus :type "AIStimulus Structure"))
  ;[1 1 1] Check if it's player, if it is, sets TargetActor with the ObjectValue. If it loses sight of us which can happen twice - when it first sees us and when it loses sight of us - when it first loses sight of us it sets TargetActor as nothing. And finally when it does lose sight of us, it will get our vector and log it as LastKnownLocation.
  (`self.HandleSightSense` Actor Stimulus)
  (`self.HandleSoundSense` Stimulus))

(fn `HandleSightSense`
  (params (Actor :type "Actor Object Reference") (Stimulus :type "AIStimulus Structure"))
  (bind (_stimulus_age _stimulus_expirationage _stimulus_strength _stimulus_stimuluslocation _stimulus_receiverlocation _stimulus_tag _stimulus_bsuccessfullysensed) (break `AIStimulus` (`local.Stimulus`)))
  (bind _returnvalue (`AIPerceptionSystem.GetSenseClassForStimulus` Stimulus))
  (if (== _returnvalue "/Script/AIModule.AISense_Sight")
    (if (== (`local.Actor`) (`GameplayStatics.GetPlayerCharacter` 0))
      (`KismetSystemLibrary.PrintString` "I found you!")
      (`BlackboardComponent.SetValueAsObject` (`self.Blackboard`) "FoundPlayer" (`KismetMathLibrary.SelectObject` (`GameplayStatics.GetPlayerCharacter` 0) null _stimulus_bsuccessfullysensed))
      (if (not _stimulus_bsuccessfullysensed)
        (`KismetSystemLibrary.PrintString` "Where did you go? I'm going to look around!")
        (`BlackboardComponent.SetValueAsVector` (`self.Blackboard`) "PlayerLastKnownLocation" _stimulus_stimuluslocation))
      (else
        (return)))
    (else
      (return))))

(fn `HandleSoundSense`
  (params (Stimulus :type "AIStimulus Structure (by ref)"))
  (bind _returnvalue (`AIPerceptionSystem.GetSenseClassForStimulus` Stimulus))
  (if (== _returnvalue "/Script/AIModule.AISense_Hearing")
    (`KismetSystemLibrary.PrintString` "I heard something.")
    (`BlackboardComponent.SetValueAsVector` (`self.Blackboard`) "HeardNoiseLocation" (`.StimulusLocation` (break `AIStimulus` (`local.Stimulus`))))))

(fn `UserConstructionScript`)