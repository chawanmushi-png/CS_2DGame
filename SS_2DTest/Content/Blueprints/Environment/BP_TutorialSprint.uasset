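; BP_TutorialSprint is a trigger volume that shows a sprint tutorial widget while the player is inside its box.
; On BeginPlay it creates WBP_TutorialSprint, adds it to the viewport and keeps it hidden.
; Player overlap makes the widget visible and plays FadeIn.
; Leaving plays FadeOut after a short delay, then hides the widget once a further delay has elapsed.
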(event `self.ReceiveBeginPlay`
  (bind _returnvalue (`|CreateWidget` "/Game/Blueprints/Environment/Widgets/WBP_TutorialSprint.WBP_TutorialSprint_C"))
  (bind _output_get (set `self.TutorialSprint` _returnvalue))
  (`UserWidget.AddToViewport` _output_get 0)
  (`Widget.SetVisibility` _output_get "Hidden"))

(event `self.Box.OnComponentBeginOverlap`
  (params (OverlappedComponent :type "PrimitiveComponent Object Reference") (OtherActor :type "Actor Object Reference") (OtherComp :type "PrimitiveComponent Object Reference") (OtherBodyIndex :type Integer) (bFromSweep :type Boolean) (SweepResult :type "HitResult Structure (by ref)"))
  (bind _tutorialsprint (`self.TutorialSprint`))
  (if (== OtherActor (`GameplayStatics.GetPlayerCharacter` 0))
    (`Widget.SetVisibility` _tutorialsprint "Visible")
    (`UserWidget.PlayAnimation` _tutorialsprint (`/Game/Blueprints/Environment/Widgets/WBP_TutorialSprint.FadeIn` _tutorialsprint) 0.0 1 "Forward" 1.0 false)))

(event `self.Box.OnComponentEndOverlap`
  (params (OverlappedComponent :type "PrimitiveComponent Object Reference") (OtherActor :type "Actor Object Reference") (OtherComp :type "PrimitiveComponent Object Reference") (OtherBodyIndex :type Integer))
  (bind _tutorialsprint (`self.TutorialSprint`))
  (if (== OtherActor (`GameplayStatics.GetPlayerCharacter` 0))
    (`KismetSystemLibrary.Delay` 0.2)
    (`UserWidget.PlayAnimation` _tutorialsprint (`/Game/Blueprints/Environment/Widgets/WBP_TutorialSprint.FadeOut` _tutorialsprint) 0.0 1 "Forward" 1.0 false)
    (`KismetSystemLibrary.Delay` 1.0)
    (`Widget.SetVisibility` (`self.TutorialSprint`) "Hidden")))

(fn `UserConstructionScript`)