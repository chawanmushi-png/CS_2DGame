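; Trigger-box exit that loads the Map_Class2DTutorial level when the player interacts inside it.
; BeginPlay creates a hidden prompt widget, which fades in on player overlap as input is enabled and a Gate opens.
; IA_Interact passes through the Gate and a DoOnce to open the level.
; Leaving fades the prompt out and closes the Gate only after the delays, calling EnableInput again rather than disabling input.
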(event `self.ReceiveBeginPlay`
  (bind _returnvalue (`|CreateWidget` "/Game/Blueprints/Environment/Widgets/WBP_TutorialExitPrompt.WBP_TutorialExitPrompt_C"))
  (bind _output_get (set `self.TutorialExitPrompt` _returnvalue))
  (`UserWidget.AddToViewport` _output_get 0)
  (`Widget.SetVisibility` _output_get "Hidden"))

(event `EnhancedInput|/Game/Blueprints/Input/Actions/IA_Interact`
  (params (ActionValue :type Boolean) (ElapsedSeconds :type "Float (double-precision)") (TriggeredSeconds :type "Float (double-precision)") (InputAction :type "InputAction Object Reference" :default "/Game/Blueprints/Input/Actions/IA_Interact.IA_Interact"))
  (:`Triggered`
    (`/Engine/EditorBlueprintResources/StandardMacros.Gate` true :!label _label
      (:`Exit`
        (`/Engine/EditorBlueprintResources/StandardMacros.DoOnce` false
          (:`Completed`
            (`GameplayStatics.OpenLevel` "Map_Class2DTutorial")))))))

(event `self.Box.OnComponentBeginOverlap`
  (params (OverlappedComponent :type "PrimitiveComponent Object Reference") (OtherActor :type "Actor Object Reference") (OtherComp :type "PrimitiveComponent Object Reference") (OtherBodyIndex :type Integer) (bFromSweep :type Boolean) (SweepResult :type "HitResult Structure (by ref)"))
  (bind _tutorialexitprompt (`self.TutorialExitPrompt`))
  (if (== OtherActor (`GameplayStatics.GetPlayerCharacter` 0))
    (`Widget.SetVisibility` _tutorialexitprompt "Visible")
    (`UserWidget.PlayAnimation` _tutorialexitprompt (`/Game/Blueprints/Environment/Widgets/WBP_TutorialExitPrompt.FadeIn` _tutorialexitprompt) 0.0 1 "Forward" 1.0 false)
    (`self.EnableInput` (`GameplayStatics.GetPlayerController` 0))
    (goto _label :!via `Open`)))

(event `self.Box.OnComponentEndOverlap`
  (params (OverlappedComponent :type "PrimitiveComponent Object Reference") (OtherActor :type "Actor Object Reference") (OtherComp :type "PrimitiveComponent Object Reference") (OtherBodyIndex :type Integer))
  (bind _tutorialexitprompt (`self.TutorialExitPrompt`))
  (if (== (`GameplayStatics.GetPlayerCharacter` 0) OtherActor)
    (`KismetSystemLibrary.Delay` 0.2)
    (`UserWidget.PlayAnimation` _tutorialexitprompt (`/Game/Blueprints/Environment/Widgets/WBP_TutorialExitPrompt.FadeOut` _tutorialexitprompt) 0.0 1 "Forward" 1.0 false)
    (`KismetSystemLibrary.Delay` 1.0)
    (`Widget.SetVisibility` _tutorialexitprompt "Hidden")
    (`self.EnableInput` (`GameplayStatics.GetPlayerController` 0))
    (goto _label :!via `Close`)))

(fn `UserConstructionScript`)