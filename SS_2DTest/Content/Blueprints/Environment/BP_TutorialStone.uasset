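; BP_TutorialStone is an environment actor that shows a tutorial dialogue box while the player is near it.
; On BeginPlay it creates its own WBP_TutorialDialogueBox, adds it to the viewport and hides it.
; When the player character enters the Box trigger the widget becomes visible and plays FadeIn.
; On exit it waits briefly, plays FadeOut, then hides the widget after a further delay.
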(event `self.ReceiveBeginPlay`
  (bind _returnvalue (`|CreateWidget` "/Game/Blueprints/Environment/Widgets/WBP_TutorialDialogueBox.WBP_TutorialDialogueBox_C"))
  (bind _output_get (set `self.TutorialWidget` _returnvalue))
  (`UserWidget.AddToViewport` _output_get 0)
  (`Widget.SetVisibility` _output_get "Hidden"))

(event `self.Box.OnComponentBeginOverlap`
  (params (OverlappedComponent :type "PrimitiveComponent Object Reference") (OtherActor :type "Actor Object Reference") (OtherComp :type "PrimitiveComponent Object Reference") (OtherBodyIndex :type Integer) (bFromSweep :type Boolean) (SweepResult :type "HitResult Structure (by ref)"))
  (bind _tutorialwidget (`self.TutorialWidget`))
  (if (== OtherActor (`GameplayStatics.GetPlayerCharacter` 0))
    (`Widget.SetVisibility` _tutorialwidget "Visible")
    (`UserWidget.PlayAnimation` _tutorialwidget (`/Game/Blueprints/Environment/Widgets/WBP_TutorialDialogueBox.FadeIn` _tutorialwidget) 0.0 1 "Forward" 1.0 false)))

(event `self.Box.OnComponentEndOverlap`
  (params (OverlappedComponent :type "PrimitiveComponent Object Reference") (OtherActor :type "Actor Object Reference") (OtherComp :type "PrimitiveComponent Object Reference") (OtherBodyIndex :type Integer))
  (bind _tutorialwidget (`self.TutorialWidget`))
  (if (== OtherActor (`GameplayStatics.GetPlayerCharacter` 0))
    (`KismetSystemLibrary.Delay` 0.2)
    (`UserWidget.PlayAnimation` _tutorialwidget (`/Game/Blueprints/Environment/Widgets/WBP_TutorialDialogueBox.FadeOut` _tutorialwidget) 0.0 1 "Forward" 1.0 false)
    (`KismetSystemLibrary.Delay` 1.0)
    (`Widget.SetVisibility` (`self.TutorialWidget`) "Hidden")))

(fn `UserConstructionScript`)