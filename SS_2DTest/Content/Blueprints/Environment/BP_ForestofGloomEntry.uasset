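; BP_ForestofGloomEntry is a trigger actor that shows a Forest of Gloom screen the first time the player enters its zone.
; On BeginPlay it creates the WBP_ForestOfGloomScreen widget, adds it to the viewport and keeps it hidden.
; When the player character overlaps the Box, it reveals the widget, sets an EnteredZone flag to prevent repeats, then hides it after a fixed delay.
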(event `self.ReceiveBeginPlay`
  (bind _returnvalue (`|CreateWidget` "/Game/Blueprints/Environment/Widgets/WBP_ForestOfGloomScreen.WBP_ForestOfGloomScreen_C"))
  (bind _output_get (set `self.ForestOfGloomWidget` _returnvalue))
  (`UserWidget.AddToViewport` _output_get 0)
  (`Widget.SetVisibility` _output_get "Hidden"))

(event `self.Box.OnComponentBeginOverlap`
  (params (OverlappedComponent :type "PrimitiveComponent Object Reference") (OtherActor :type "Actor Object Reference") (OtherComp :type "PrimitiveComponent Object Reference") (OtherBodyIndex :type Integer) (bFromSweep :type Boolean) (SweepResult :type "HitResult Structure (by ref)"))
  (bind _forestofgloomwidget (`self.ForestOfGloomWidget`))
  (if (== OtherActor (`GameplayStatics.GetPlayerCharacter` 0))
    (if (not (`self.EnteredZone`))
      (`Widget.SetVisibility` _forestofgloomwidget "Visible")
      (set `self.EnteredZone` true)
      (`KismetSystemLibrary.Delay` 8.0)
      (`Widget.SetVisibility` _forestofgloomwidget "Hidden"))))

(fn `UserConstructionScript`)