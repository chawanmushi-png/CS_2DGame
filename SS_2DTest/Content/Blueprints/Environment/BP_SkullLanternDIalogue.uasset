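; Skull lantern pickup that gives the player's BP_Warrior a visible lantern and shows a one-time dialogue.
; BeginPlay hides the warrior's lantern flipbook and light.
; Overlapping LanternBox reveals them and hides this actor's own flipbook and light, once.
; A separate DialogueBox fades in WBP_SkullLanternDialogue on entry, then on exit fades it out, removes it after a delay and blocks repeats.
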(event `self.ReceiveBeginPlay`
  (bind _asbp_warrior (cast `/Game/Blueprints/Warrior/BP_Warrior` (`GameplayStatics.GetPlayerCharacter` 0)))
  (bind _output_get (set `self.As BP Warrior` _asbp_warrior))
  (`SceneComponent.SetVisibility` (`/Game/Blueprints/Warrior/BP_Warrior.Lantern FlipBook` _output_get) false false)
  (`SceneComponent.SetVisibility` (`/Game/Blueprints/Warrior/BP_Warrior.LanternPointLight` _output_get) false false))

(event `self.LanternBox.OnComponentBeginOverlap`
  (params (OverlappedComponent :type "PrimitiveComponent Object Reference") (OtherActor :type "Actor Object Reference") (OtherComp :type "PrimitiveComponent Object Reference") (OtherBodyIndex :type Integer) (bFromSweep :type Boolean) (SweepResult :type "HitResult Structure (by ref)"))
  (bind _as_bp_warrior (`self.As BP Warrior`))
  (if (`self.SkullIsTriggered`)
    _
    (elif (== OtherActor (`GameplayStatics.GetPlayerCharacter` 0))
      (`SceneComponent.SetVisibility` (`/Game/Blueprints/Warrior/BP_Warrior.Lantern FlipBook` _as_bp_warrior) true false)
      (`SceneComponent.SetVisibility` (`/Game/Blueprints/Warrior/BP_Warrior.LanternPointLight` _as_bp_warrior) true false)
      (`SceneComponent.SetVisibility` (`self.PaperFlipbook`) false false)
      (`SceneComponent.SetVisibility` (`self.PointLight`) false false)
      (set `self.SkullIsTriggered` true))))

(event `self.DialogueBox.OnComponentBeginOverlap`
  (params (OverlappedComponent :type "PrimitiveComponent Object Reference") (OtherActor :type "Actor Object Reference") (OtherComp :type "PrimitiveComponent Object Reference") (OtherBodyIndex :type Integer) (bFromSweep :type Boolean) (SweepResult :type "HitResult Structure (by ref)"))
  (if (`self.DialogueIsTriggered`)
    _
    (elif (== (`GameplayStatics.GetPlayerCharacter` 0) OtherActor)
      (bind _returnvalue (`|CreateWidget` "/Game/Blueprints/Environment/Widgets/WBP_SkullLanternDialogue.WBP_SkullLanternDialogue_C"))
      (`UserWidget.AddToViewport` _returnvalue 0)
      (`UserWidget.PlayAnimation` _returnvalue (`/Game/Blueprints/Environment/Widgets/WBP_SkullLanternDialogue.FadeIn` _returnvalue) 0.0 1 "Forward" 1.0 false))))

(event `self.DialogueBox.OnComponentEndOverlap`
  (params (OverlappedComponent :type "PrimitiveComponent Object Reference") (OtherActor :type "Actor Object Reference") (OtherComp :type "PrimitiveComponent Object Reference") (OtherBodyIndex :type Integer))
  (if (`self.DialogueIsTriggered`)
    _
    (elif (== (`GameplayStatics.GetPlayerCharacter` 0) OtherActor)
      (`UserWidget.PlayAnimation` (stale `self.DialogueBox.OnComponentBeginOverlap` _returnvalue) (`/Game/Blueprints/Environment/Widgets/WBP_SkullLanternDialogue.FadeOut` (stale `self.DialogueBox.OnComponentBeginOverlap` _returnvalue)) 0.0 1 "Forward" 1.0 false)
      (`KismetSystemLibrary.Delay` 1.0)
      (`Widget.RemoveFromParent` (stale `self.DialogueBox.OnComponentBeginOverlap` _returnvalue))
      (set `self.DialogueIsTriggered` true))))

(fn `UserConstructionScript`)